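; Enemy AI character with melee sword attacks, stealth-assassination victim behavior and camera-facing overhead widgets.
; Behavior-tree attacks drive a montage combo via AttackIndex and buffered input, with timer-looped sword and one-shot kick/stab sphere traces damaging "Damageable" actors.
; Player proximity shows the assassination prompt; assassination plays a victim montage, then delayed ragdoll.
; Any damage launches and immediately ragdolls it, as health reduction is disconnected.
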(event OnComponentBeginOverlap(AssassinationRedius)
  (params (OverlappedComponent :type Primitive%20Component%20Object%20Reference) (OtherActor :type Actor%20Object%20Reference) (OtherComp :type Primitive%20Component%20Object%20Reference) (OtherBodyIndex :type Integer) (bFromSweep :type Boolean) (SweepResult :type Hit%20Result%20Structure%20%28by%20ref%29))
  (Utilities|Casting|CastToBPC_Player OtherActor)
  (Rendering|SetVisibility (Variables|Default|GetUI_Assasinate%20Widget) true false))

(event OnComponentEndOverlap(AssassinationRedius)
  (params (OverlappedComponent :type Primitive%20Component%20Object%20Reference) (OtherActor :type Actor%20Object%20Reference) (OtherComp :type Primitive%20Component%20Object%20Reference) (OtherBodyIndex :type Integer))
  (Utilities|Casting|CastToBPC_Player OtherActor)
  (Rendering|SetVisibility (Variables|Default|GetUI_Assasinate%20Widget) false false))

(event Custom|SwordAttack
  ;[0.2232 0.227 0.2232] Combo System
  ;;[0.2232 0.227 0.2232] Sword attack
  (if (Variables|Default|GetIsAttacking)
    (Variables|Default|SetSaveAttack? true)
    (else
      (Variables|Default|SetIsAttacking true)
      (switch int (Variables|Default|GetAttackIndex)
        (:0
          (CallFunction|Attack1))
        (:1
          (CallFunction|Attack2))
        (:2
          (CallFunction|Attack4))))))

(event Custom|SwordAttackCombo
  ;[0.2232 0.227 0.2232] Combo System
  ;;[0.2232 0.227 0.2232] ComboContinue
  (if (Variables|Default|GetSaveAttack?)
    (Variables|Default|SetSaveAttack? false)
    (switch int (Variables|Default|GetAttackIndex)
      (:0
        (CallFunction|Attack1))
      (:1
        (CallFunction|Attack2))
      (:2
        (CallFunction|Attack4)))
    (else
      (CallFunction|StopCombo))))

(event Custom|Sword%20Trace%20Loop
  ;[0.2232 0.227 0.2232] Sword Trace
  (bind (_outhit _returnvalue) (Collision|SphereTraceByChannel (Transformation|GetWorldLocation (Variables|Default|GetSwordTopPoint)) (Transformation|GetWorldLocation (Variables|Default|GetSwordBottomPoint)) 2e+01 "TraceTypeQuery1" false 0 "ForDuration" true "(R=1.000000,G=0.000000,B=0.000000,A=1.000000)" "(R=0.000000,G=1.000000,B=0.000000,A=1.000000)" 0.2))
  (if _returnvalue
    (if (Actor|ActorHasTag (.HitActor (Collision|BreakHitResult _outhit)) "Damageable")
      (Utilities|FlowControl|DoOnce false :!label _label
        (:Completed
          (Game|Damage|ApplyDamage (.HitActor (Collision|BreakHitResult _outhit)) (Variables|Default|GetBase%20Damage%20To%20Apply) 0 0)
          (Camera|PlayWorldCameraShake "/Game/Blueprints/Other/CS_HitCameraShake.CS_HitCameraShake_C" (.Location (Collision|BreakHitResult _outhit)) 0.0 2e+03)
          (CallFunction|PlaySwordHitSound)
          (Effects|SpawnEmitteratLocation "/Game/Assets/Particles/Blood/P_Blood_Splat_Cone.P_Blood_Splat_Cone" (.Location (Collision|BreakHitResult _outhit)) (Math|Rotator|MakeRotfromXY (.Normal (Collision|BreakHitResult _outhit)) (.Normal (Collision|BreakHitResult _outhit))) "0.400000,0.400000,0.400000")
          (Utilities|FlowControl|Delay 0.5)
          (goto _label Reset))))))

(event Custom|Stop%20Sword%20Trace
  ;[0.2232 0.227 0.2232] Sword Trace
  (Utilities|Time|ClearandInvalidateTimerbyHandle (Variables|Default|GetSwordTraceLoop)))

(event Custom|Sphere%20Trace%20For%20stabb%20and%20kick
  (bind _sphere_trace_pos (Variables|Default|GetSphere%20Trace%20Pos))
  (bind _returnvalue (Transformation|GetWorldLocation _sphere_trace_pos))
  ;[0.2232 0.227 0.2232] Sphere trace for kick and stabb
  (bind (_outhit _returnvalue_2) (Collision|SphereTraceByChannel _returnvalue _returnvalue 25.0 "TraceTypeQuery1" false 0 "ForDuration"))
  (if _returnvalue_2
    (if (Actor|ActorHasTag (.HitActor (Collision|BreakHitResult _outhit)) "Damageable")
      (Game|Damage|ApplyDamage (.HitActor (Collision|BreakHitResult _outhit)) (Variables|Default|GetBase%20Damage%20To%20Apply) 0 0)
      (Camera|PlayWorldCameraShake "/Game/Blueprints/Other/CS_HitCameraShake.CS_HitCameraShake_C" (.Location (Collision|BreakHitResult _outhit)) 0.0 2e+03)
      (CallFunction|PlaySwordHitSound)
      (Effects|SpawnEmitteratLocation "/Game/Assets/Particles/Blood/P_Blood_Splat_Cone.P_Blood_Splat_Cone" (.Location (Collision|BreakHitResult _outhit)) (Math|Rotator|MakeRotfromXY (.ImpactNormal (Collision|BreakHitResult _outhit)) (.ImpactNormal (Collision|BreakHitResult _outhit))) "0.400000,0.400000,0.400000"))))

(event Custom|Ragdoll
  ;[0.01938 0.01938 0.01938] Ragdoll
  (Utilities|FlowControl|Sequence
    (:then_0
      (Utilities|FlowControl|Delay 2.5)
      (Physics|SetSimulatePhysics (Variables|Character|GetMesh) true))
    (:then_1
      (Utilities|FlowControl|Delay 1.8)
      (Audio|PlaySoundatLocation "/Game/Assets/Audio/Grunts_hits/SC_Death.SC_Death" (Transformation|GetActorLocation) "0, 0, 0" 1.0 1.0 0.0 "/Game/Assets/Audio/Footsteps/SA_Character.SA_Character" 0 0 0))))

(event Custom|Attack%202
  ;[0.2232 0.227 0.2232] Combo System
  ;;[0.2232 0.227 0.2232] Attack 2
  (Utilities|FlowControl|DoOnce false :!label _label
    (:Completed
      (Utilities|FlowControl|Delay 0.1)
      (Animation|Montage|PlayMontage (Variables|Character|GetMesh) "/Game/Assets/CharacterAnimations/SwordAttack/ANM_Attack2.ANM_Attack2"
        (:then
          (Variables|Default|SetAttackIndex 2)
          (goto _label Reset))))))

(event Custom|Attack1
  ;[0.2232 0.227 0.2232] Combo System
  ;;[0.2232 0.227 0.2232] Attack 1
  (Utilities|FlowControl|DoOnce false :!label _label
    (:Completed
      (Utilities|FlowControl|Delay 0.1)
      (Animation|Montage|PlayMontage (Variables|Character|GetMesh) "/Game/Assets/CharacterAnimations/SwordAttack/ANM_Attack1.ANM_Attack1"
        (:then
          (Variables|Default|SetAttackIndex 1)
          (goto _label Reset))))))

(event Custom|StopCombo
  ;[0.2232 0.227 0.2232] Combo System
  ;;[0.2232 0.227 0.2232] Stop combo / attack
  (Variables|Default|SetIsAttacking false)
  (Variables|Default|SetAttackIndex 0))

(event Custom|Attack%204
  ;[0.2232 0.227 0.2232] Combo System
  ;;[0.2232 0.227 0.2232] Attack 1
  (Utilities|FlowControl|DoOnce false :!label _label
    (:Completed
      (Utilities|FlowControl|Delay 0.1)
      (Animation|Montage|PlayMontage (Variables|Character|GetMesh) "/Game/Assets/CharacterAnimations/SwordAttack/ANM_Attack3.ANM_Attack3"
        (:then
          (Variables|Default|SetAttackIndex 4)
          (goto _label Reset))))))

(event Custom|Play%20sword%20hit%20sound
  ;[0.2232 0.227 0.2232] play sword hit sound
  (Audio|PlaySoundatLocation "/Game/Assets/Audio/MeleeWapons/MS_SwordAttackHit.MS_SwordAttackHit" (Transformation|GetActorLocation (Components|GetOwner)) "0, 0, 0" 1.0 1.0 0.0 0 0 0 0))

(event Custom|Sword%20Attack%20combo%20call%20from%20BT
  ;[0.2232 0.227 0.2232] Combo System
  ;;[0.2232 0.227 0.2232] Attack input
  (if (Variables|Default|GetCanAttack)
    (CallFunction|SwordAttack)))

(event Custom|Enable%20Investigate%20Icon
  (Utilities|FlowControl|FlipFlop
    (:A
      (Rendering|SetVisibility (Variables|Default|GetUI_InvestigatIcon) true false))
    (:B
      (Rendering|SetVisibility (Variables|Default|GetUI_InvestigatIcon) false false))))

(event Custom|Attack%203
  ;[0.2232 0.227 0.2232] Combo System
  ;;[0.2232 0.227 0.2232] Attack 3
  (Utilities|FlowControl|DoOnce false :!label _label
    (:Completed
      (Utilities|FlowControl|Delay 0.1)
      (Animation|Montage|PlayMontage (Variables|Character|GetMesh) "/Game/Assets/CharacterAnimations/SwordAttack/ANM_Kick.ANM_Kick"
        (:then
          (Variables|Default|SetAttackIndex 3)
          (goto _label Reset))))))

(event Custom|Start%20Sword%20Trace
  ;[0.2232 0.227 0.2232] Sword Trace
  (bind _returnvalue (Utilities|Time|SetTimerbyEvent (delegate Custom|Sword%20Trace%20Loop) 0.001 true))
  (Variables|Default|SetSwordTraceLoop _returnvalue))

(event Collision|EventActorBeginOverlap
  (params (OtherActor :type Actor%20Object%20Reference)))

(event EventTick
  (params (DeltaSeconds :type Float%20%28single-precision%29))
  (Transformation|SetWorldRotation (Variables|Default|GetUI_Assasinate%20Widget) (Math|Rotator|FindLookatRotation (Transformation|GetWorldLocation (Variables|Default|GetUI_Assasinate%20Widget)) (Transformation|GetWorldLocation (Variables|/Script/Engine.PlayerCameraManager|GetTransformComponent (Game|GetPlayerCameraManager 0)))) false false))

(event Game|Damage|EventAnyDamage
  (params (Damage :type Float%20%28single-precision%29) (DamageType :type Damage%20Type%20Object%20Reference) (InstigatedBy :type Controller%20Object%20Reference) (DamageCauser :type Actor%20Object%20Reference))
  (bind _hitreactmontage (Variables|Default|GetHitReactMontage))
  (Animation|PlayAnimMontage (Utilities|Array|Get(acopy) _hitreactmontage (Math|Random|RandomIntegerinRange 0 (- (Utilities|Array|Length _hitreactmontage) 1))) 1.0 "None")
  (bind _asbpc_player (Utilities|Casting|CastToBPC_Player (Game|GetPlayerCharacter 0)))
  (Character|LaunchCharacter (* (Math|Vector|GetForwardVector (Transformation|GetActorRotation _asbpc_player)) 8.5e+02) false false)
  (Audio|PlaySoundatLocation "/Game/Assets/Audio/Grunts_hits/416838__tonsil5__grunt2-death-pain.416838__tonsil5__grunt2-death-pain" (Transformation|GetActorLocation) "0, 0, 0" 1.0 (Math|Random|RandomFloatinRange 0.8 1.3) 0.0 0 0 0 0)
  (if true
    (Collision|SetCollisionObjectType (Variables|Character|GetMesh) "ECC_PhysicsBody")
    (Physics|SetSimulatePhysics (Variables|Character|GetMesh) true)
    (Audio|PlaySoundatLocation "/Game/Assets/Audio/Grunts_hits/SC_Death.SC_Death" (Transformation|GetActorLocation) "0, 0, 0" 1.0 1.0 0.0 0 0 0 0)
    (Rendering|SetVisibility (Variables|Default|GetUI_HealthBar) false false)))

(event EventBeginPlay
  (bind _aswbp_enemy_healthbar (Utilities|Casting|CastToWBP_NPC_Healthbar (UserInterface|GetWidget (Variables|Default|GetUI_HealthBar))))
  (Variables|Default|SetUI%20Enemy%20Health _aswbp_enemy_healthbar))

(fn ConstructionScript)

(fn Attack
  (CallFunction|SwordAttackComboCallfromBT)
  (return 0.4))

(fn StealthBackAssissinate
  (Animation|PlayAnimMontage "/Game/Assets/CharacterAnimations/Assassinations/ANM_Paired_Knife_Stealth_KidneyAndNeck_Victim.ANM_Paired_Knife_Stealth_KidneyAndNeck_Victim" 1.0 "None")
  (CallFunction|Ragdoll)
  (Rendering|SetVisibility (Variables|Default|GetUI_Assasinate%20Widget) false false)
  (return (Transformation|GetWorldLocation (Variables|Default|GetAssassin%20Ref)) (Transformation|GetActorRotation)))