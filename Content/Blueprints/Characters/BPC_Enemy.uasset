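; Enemy character that can be stealth-assassinated from behind by the player.
; An overlap radius shows an assassination prompt widget while BPC_Player is inside, and Tick turns it toward the player camera.
; StealthBackAssissinate plays the victim's paired knife montage, hides the prompt and returns a reference location and the enemy's rotation for the attacker.
; It also fires Ragdoll, which uses timed delays to play the death sound, then enable mesh physics.
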(event OnComponentBeginOverlap(AssassinationRedius)
  (params (OverlappedComponent :type Primitive%20Component%20Object%20Reference) (OtherActor :type Actor%20Object%20Reference) (OtherComp :type Primitive%20Component%20Object%20Reference) (OtherBodyIndex :type Integer) (bFromSweep :type Boolean) (SweepResult :type Hit%20Result%20Structure%20%28by%20ref%29))
  (Utilities|Casting|CastToBPC_Player OtherActor)
  (Rendering|SetVisibility (Variables|Default|GetAssasinate%20Widget) true false))

(event OnComponentEndOverlap(AssassinationRedius)
  (params (OverlappedComponent :type Primitive%20Component%20Object%20Reference) (OtherActor :type Actor%20Object%20Reference) (OtherComp :type Primitive%20Component%20Object%20Reference) (OtherBodyIndex :type Integer))
  (Utilities|Casting|CastToBPC_Player OtherActor)
  (Rendering|SetVisibility (Variables|Default|GetAssasinate%20Widget) false false))

(event Custom|Ragdoll
  ;[0.01938 0.01938 0.01938] Ragdoll
  (Utilities|FlowControl|Sequence
    (:then_0
      (Utilities|FlowControl|Delay 2.5)
      (Physics|SetSimulatePhysics (Variables|Character|GetMesh) true))
    (:then_1
      (Utilities|FlowControl|Delay 1.8)
      (Audio|PlaySoundatLocation "/Game/Assets/Audio/Grunts_hits/SC_Death.SC_Death" (Transformation|GetActorLocation) "0, 0, 0" 1.0 1.0 0.0 "/Game/Assets/Audio/Footsteps/SA_Character.SA_Character" 0 0 0))))

(event EventBeginPlay)

(event Collision|EventActorBeginOverlap
  (params (OtherActor :type Actor%20Object%20Reference)))

(event EventTick
  (params (DeltaSeconds :type Float%20%28single-precision%29))
  (Transformation|SetWorldRotation (Variables|Default|GetAssasinate%20Widget) (Math|Rotator|FindLookatRotation (Transformation|GetWorldLocation (Variables|Default|GetAssasinate%20Widget)) (Transformation|GetWorldLocation (Variables|/Script/Engine.PlayerCameraManager|GetTransformComponent (Game|GetPlayerCameraManager 0)))) false false))

(fn ConstructionScript)

(fn StealthBackAssissinate
  (Animation|PlayAnimMontage "/Game/Assets/PlayerAnimation/Assassinations/ANM_Paired_Knife_Stealth_KidneyAndNeck_Victim.ANM_Paired_Knife_Stealth_KidneyAndNeck_Victim" 1.0 "None")
  (CallFunction|Ragdoll)
  (Rendering|SetVisibility (Variables|Default|GetAssasinate%20Widget) false false)
  (return (Transformation|GetWorldLocation (Variables|Default|GetAssassin%20Ref)) (Transformation|GetActorRotation)))