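; BPC_Troop is an AI troop character that follows the player or moves to an ordered location, and can be stealth-assassinated from behind.
; A delayed self-calling FollowPlayer loop chases beyond a set distance; TroopMoveTo clears the follow flag.
; Tick turns the health bar and assassination widget toward the camera.
; StealthBackAssissinate plays the victim montage, triggers delayed ragdoll and death sound, and returns alignment transforms; damage-reaction logic is disconnected.
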(event Custom|Ragdoll
  ;[0.01938 0.01938 0.01938] Ragdoll
  (Utilities|FlowControl|Sequence
    (:then_0
      (Utilities|FlowControl|Delay 2.5)
      (Physics|SetSimulatePhysics (Variables|Character|GetMesh) true))
    (:then_1
      (Utilities|FlowControl|Delay 1.8)
      (Audio|PlaySoundatLocation "/Game/Assets/Audio/Grunts_hits/SC_Death.SC_Death" (Transformation|GetActorLocation) "0, 0, 0" 1.0 1.0 0.0 "/Game/Assets/Audio/Footsteps/SA_Character.SA_Character" 0 0 0))))

(event Custom|Follow%20Player
  ;[0.2232 0.227 0.2232] Troop Recive Oder from player
  ;;[0.2232 0.227 0.2232] Troop Follow Player
  (if (Variables|Default|GetFollowPlayer)
    (if (>= (Transformation|GetDistanceTo (Variables|Default|GetAs%20BPC%20Player)) 4e+02)
      (AI|AIMoveTo self "0, 0, 0" (Variables|Default|GetAs%20BPC%20Player) 5.0 false
        (:then
          _))
      (else
        (AI|AIMoveTo self "0, 0, 0" self 5.0 false
          (:then
            _))))
    (Utilities|FlowControl|Delay 0.2)
    (CallFunction|FollowPlayer)))

(event Custom|Stop%20Movements
  ;[0.2232 0.227 0.2232] Troop Recive Oder from player
  ;;[0.2232 0.227 0.2232] Troop Follow Player
  (AI|AIMoveTo self "0, 0, 0" self 5.0 false
    (:then
      (Utilities|FlowControl|Delay 0.2)
      (CallFunction|FollowPlayer))))

(event Custom|Troop%20Move%20To
  (params (Destination :type Vector))
  ;[0.2232 0.227 0.2232] Troop Recive Oder from player
  ;;[0.2232 0.227 0.2232] Troop Move to locatin
  (Variables|Default|SetFollowPlayer false)
  (AI|AIMoveTo self Destination 0 5.0 false))

(event Collision|EventActorBeginOverlap
  (params (OtherActor :type Actor%20Object%20Reference)))

(event EventTick
  (params (DeltaSeconds :type Float%20%28single-precision%29))
  (bind _returnvalue (Game|GetPlayerCameraManager 0))
  (bind _assasinate_widget (Variables|Default|GetAssasinate%20Widget))
  (bind _returnvalue_2 (Transformation|GetWorldLocation _assasinate_widget))
  (bind _transformcomponent (Variables|/Script/Engine.PlayerCameraManager|GetTransformComponent _returnvalue))
  (bind _returnvalue_3 (Transformation|GetWorldLocation _transformcomponent))
  (bind _returnvalue_4 (Math|Rotator|FindLookatRotation _returnvalue_2 _returnvalue_3))
  (Transformation|SetWorldRotation (Variables|Default|GetAssasinate%20Widget) _returnvalue_4 false false)
  (Transformation|SetWorldRotation (Variables|Default|GetHealthBar) _returnvalue_4 false false))

(event Game|Damage|EventAnyDamage
  (params (Damage :type Float%20%28single-precision%29) (DamageType :type Damage%20Type%20Object%20Reference) (InstigatedBy :type Controller%20Object%20Reference) (DamageCauser :type Actor%20Object%20Reference)))

(event EventBeginPlay
  (bind _aswbp_npc_healthbar (Utilities|Casting|CastToWBP_NPC_Healthbar (UserInterface|GetWidget (Variables|Default|GetHealthBar))))
  (Variables|Default|SetUI%20Enemy%20Health _aswbp_npc_healthbar)
  (bind _asbpc_player (Utilities|Casting|CastToBPC_Player (Game|GetPlayerCharacter 0)))
  (Variables|Default|SetAs%20BPC%20Player _asbpc_player)
  (CallFunction|FollowPlayer))

(fn ConstructionScript)

(fn StealthBackAssissinate
  (Animation|PlayAnimMontage "/Game/Assets/CharacterAnimations/Assassinations/ANM_Paired_Knife_Stealth_KidneyAndNeck_Victim.ANM_Paired_Knife_Stealth_KidneyAndNeck_Victim" 1.0 "None")
  (CallFunction|Ragdoll)
  (Rendering|SetVisibility (Variables|Default|GetAssasinate%20Widget) false false)
  (return (Transformation|GetWorldLocation (Variables|Default|GetAssassin%20Ref)) (Transformation|GetActorRotation)))