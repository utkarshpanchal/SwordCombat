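; BPC_Dummy is an enemy dummy character that can be damaged or stealth-assassinated by the player.
; Health bar and assassination prompt face the camera each tick, with the prompt shown while the player overlaps a radius.
; Damage triggers random hit reactions and knockback along player facing, feeding CompPlayerState, which signals death for ragdoll.
; StealthBackAssissinate plays the victim montage, triggers delayed ragdoll and death sound, and returns attacker alignment location and rotation.
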(event OnComponentBeginOverlap(AssassinationRedius)
  (params (OverlappedComponent :type Primitive%20Component%20Object%20Reference) (OtherActor :type Actor%20Object%20Reference) (OtherComp :type Primitive%20Component%20Object%20Reference) (OtherBodyIndex :type Integer) (bFromSweep :type Boolean) (SweepResult :type Hit%20Result%20Structure%20%28by%20ref%29))
  (Utilities|Casting|CastToBPC_Player OtherActor)
  (Rendering|SetVisibility (Variables|Default|GetAssasinate%20Widget) true false))

(event OnComponentEndOverlap(AssassinationRedius)
  (params (OverlappedComponent :type Primitive%20Component%20Object%20Reference) (OtherActor :type Actor%20Object%20Reference) (OtherComp :type Primitive%20Component%20Object%20Reference) (OtherBodyIndex :type Integer))
  (Utilities|Casting|CastToBPC_Player OtherActor)
  (Rendering|SetVisibility (Variables|Default|GetAssasinate%20Widget) false false))

(event Custom|Ragdoll
  ;[0.01938 0.01938 0.01938] Ragdoll
  (Utilities|FlowControl|Sequence
    (:then_0
      (Utilities|FlowControl|Delay 2.5)
      (Physics|SetSimulatePhysics (Variables|Character|GetMesh) true))
    (:then_1
      (Utilities|FlowControl|Delay 1.8)
      (Audio|PlaySoundatLocation "/Game/Assets/Audio/Grunts_hits/SC_Death.SC_Death" (Transformation|GetActorLocation) "0, 0, 0" 1.0 1.0 0.0 "/Game/Assets/Audio/Footsteps/SA_Character.SA_Character" 0 0 0))))

(event Collision|EventActorBeginOverlap
  (params (OtherActor :type Actor%20Object%20Reference)))

(event EventTick
  (params (DeltaSeconds :type Float%20%28single-precision%29))
  (bind _returnvalue (Game|GetPlayerCameraManager 0))
  (bind _assasinate_widget (Variables|Default|GetAssasinate%20Widget))
  (bind _returnvalue_2 (Transformation|GetWorldLocation _assasinate_widget))
  (bind _transformcomponent (Variables|/Script/Engine.PlayerCameraManager|GetTransformComponent _returnvalue))
  (bind _returnvalue_3 (Transformation|GetWorldLocation _transformcomponent))
  (bind _returnvalue_4 (Math|Rotator|FindLookatRotation _returnvalue_2 _returnvalue_3))
  (Transformation|SetWorldRotation (Variables|Default|GetAssasinate%20Widget) _returnvalue_4 false false)
  (Transformation|SetWorldRotation (Variables|Default|GetHealthBar) _returnvalue_4 false false))

(event Game|Damage|EventAnyDamage
  (params (Damage :type Float%20%28single-precision%29) (DamageType :type Damage%20Type%20Object%20Reference) (InstigatedBy :type Controller%20Object%20Reference) (DamageCauser :type Actor%20Object%20Reference))
  (bind _hitreactmontage (Variables|Default|GetHitReactMontage))
  (Animation|PlayAnimMontage (Utilities|Array|Get(acopy) _hitreactmontage (Math|Random|RandomIntegerinRange 0 (- (Utilities|Array|Length _hitreactmontage) 1))) 1.0 "None")
  (bind _asbpc_player (Utilities|Casting|CastToBPC_Player (Game|GetPlayerCharacter 0)))
  (Character|LaunchCharacter (* (Math|Vector|GetForwardVector (Transformation|GetActorRotation _asbpc_player)) 8.5e+02) false false)
  (Audio|PlaySoundatLocation "/Game/Assets/Audio/Grunts_hits/416838__tonsil5__grunt2-death-pain.416838__tonsil5__grunt2-death-pain" (Transformation|GetActorLocation) "0, 0, 0" 1.0 (Math|Random|RandomFloatinRange 0.8 1.3) 0.0 0 0 0 0)
  (bind _isplayerdead_ (Default|DecreaseHealth (Variables|Default|GetComp_PlayerState) Damage))
  (if _isplayerdead_
    (Physics|SetSimulatePhysics (Variables|Character|GetMesh) true)
    (Audio|PlaySoundatLocation "/Game/Assets/Audio/Grunts_hits/SC_Death.SC_Death" (Transformation|GetActorLocation) "0, 0, 0" 1.0 1.0 0.0 0 0 0 0)
    (Rendering|SetVisibility (Variables|Default|GetHealthBar) false false)))

(event EventBeginPlay
  (bind _aswbp_enemy_healthbar (Utilities|Casting|CastToWBP_NPC_Healthbar (UserInterface|GetWidget (Variables|Default|GetHealthBar))))
  (Variables|Default|SetUI%20Enemy%20Health _aswbp_enemy_healthbar))

(fn ConstructionScript)

(fn StealthBackAssissinate
  (Animation|PlayAnimMontage "/Game/Assets/CharacterAnimations/Assassinations/ANM_Paired_Knife_Stealth_KidneyAndNeck_Victim.ANM_Paired_Knife_Stealth_KidneyAndNeck_Victim" 1.0 "None")
  (CallFunction|Ragdoll)
  (Rendering|SetVisibility (Variables|Default|GetAssasinate%20Widget) false false)
  (return (Transformation|GetWorldLocation (Variables|Default|GetAssassin%20Ref)) (Transformation|GetActorRotation)))