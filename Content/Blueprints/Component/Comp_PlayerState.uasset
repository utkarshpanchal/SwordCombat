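; Player state component that holds the player's current and maximum health and stamina.
; Decrease functions subtract an amount without clamping and return a depletion flag, while increase functions raise only the maximum values.
; DecreaseStamina bases its returned flag on CurrentHealth rather than CurrentStamina.
; BeginPlay and Tick are unused, so all changes come through calls to these functions.
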(event EventBeginPlay)

(event EventTick
  (params (DeltaSeconds :type Float%20%28single-precision%29)))

(fn DecreaseHealth
  (params (Damage :type Float%20%28double-precision%29))
  (Variables|Health|SetCurrentHealth (- (Variables|Health|GetCurrentHealth) Damage))
  (if (<= (Variables|Health|GetCurrentHealth) 0.0)
    (return true)
    (else
      (return false))))

(fn IncreaseMaxHealth
  (params (Health%20Incremention :type Float%20%28double-precision%29))
  (Variables|Health|SetMaxHealth (+ (Variables|Health|GetMaxHealth) Health%20Incremention)))

(fn DecreaseStamina
  (params (StaminaDepleted :type Float%20%28double-precision%29))
  (Variables|Stamina|SetCurrentStamina (- (Variables|Stamina|GetCurrentStamina) StaminaDepleted))
  (if (<= (Variables|Health|GetCurrentHealth) 0.0)
    (return true)
    (else
      (return false))))

(fn IncreaseMaxStamina
  (params (Added%20Stamina :type Float%20%28double-precision%29))
  (Variables|Stamina|SetMaxStamina (+ (Variables|Stamina|GetMaxStamina) Added%20Stamina)))