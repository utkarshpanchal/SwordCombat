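; Player combat component that runs a four-step sword and kick melee combo from the attack input.
; Presses during an attack are buffered, and SwordAttackCombo, called externally, either plays the next montage by AttackIndex or resets the combo.
; A looping timer sphere-traces along the blade with a hit cooldown, while a separate single trace covers kick and stab.
; Hits on Damageable-tagged actors apply damage, camera shake, sound and blood effects.
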(event Custom|SwordAttack
  ;[0.2232 0.227 0.2232] Combo System
  ;;[0.2232 0.227 0.2232] Sword attack
  (if (Variables|Default|GetIsAttacking)
    (Variables|Default|SetSaveAttack? true)
    (else
      (Variables|Default|SetIsAttacking true)
      (switch int (Variables|Default|GetAttackIndex)
        (:0
          (CallFunction|Attack1))
        (:1
          (CallFunction|Attack2))
        (:2
          (CallFunction|Attack3))
        (:3
          (CallFunction|Attack4))))))

(event Custom|SwordAttackCombo
  ;[0.2232 0.227 0.2232] Combo System
  ;;[0.2232 0.227 0.2232] ComboContinue
  (if (Variables|Default|GetSaveAttack?)
    (Variables|Default|SetSaveAttack? false)
    (switch int (Variables|Default|GetAttackIndex)
      (:0
        (CallFunction|Attack1))
      (:1
        (CallFunction|Attack2))
      (:2
        (CallFunction|Attack3))
      (:3
        (CallFunction|Attack4)))
    (else
      (CallFunction|StopCombo))))

(event Custom|Sword%20Trace%20Loop
  ;[0.2232 0.227 0.2232] Sword Trace
  (bind (_outhit _returnvalue) (Collision|SphereTraceByChannel (Transformation|GetWorldLocation (Variables|/Game/Blueprints/Characters/BPC_Player.BPC_Player_C|GetSwordTopPoint (Variables|Default|GetAs%20BPC%20Player))) (Transformation|GetWorldLocation (Variables|/Game/Blueprints/Characters/BPC_Player.BPC_Player_C|GetSwordBottomPoint (Variables|Default|GetAs%20BPC%20Player))) 2e+01 "TraceTypeQuery1" false 0 "None" true "(R=1.000000,G=0.000000,B=0.000000,A=1.000000)" "(R=0.000000,G=1.000000,B=0.000000,A=1.000000)" 0.2))
  (if _returnvalue
    (if (Actor|ActorHasTag (.HitActor (Collision|BreakHitResult _outhit)) "Damageable")
      (Utilities|FlowControl|DoOnce false :!label _label
        (:Completed
          (Game|Damage|ApplyDamage (.HitActor (Collision|BreakHitResult _outhit)) (Variables|Default|GetBase%20Damage%20To%20Apply) 0 0)
          (Camera|PlayWorldCameraShake "/Game/Blueprints/Other/CS_HitCameraShake.CS_HitCameraShake_C" (.Location (Collision|BreakHitResult _outhit)) 0.0 2e+03)
          (CallFunction|PlaySwordHitSound)
          (Effects|SpawnEmitteratLocation "/Game/Assets/Particles/Blood/P_Blood_Splat_Cone.P_Blood_Splat_Cone" (.Location (Collision|BreakHitResult _outhit)) (Math|Rotator|MakeRotfromXY (.Normal (Collision|BreakHitResult _outhit)) (.Normal (Collision|BreakHitResult _outhit))) "0.400000,0.400000,0.400000")
          (Utilities|FlowControl|Delay 0.5)
          (goto _label Reset))))))

(event Custom|Stop%20Sword%20Trace
  ;[0.2232 0.227 0.2232] Sword Trace
  (Utilities|Time|ClearandInvalidateTimerbyHandle (Variables|Default|GetSwordTraceLoop)))

(event Custom|Sphere%20Trace%20For%20stabb%20and%20kick
  (bind _as_bpc_player (Variables|Default|GetAs%20BPC%20Player))
  (bind _speretrace (Variables|/Game/Blueprints/Characters/BPC_Player.BPC_Player_C|GetSpereTrace _as_bpc_player))
  (bind _returnvalue (Transformation|GetWorldLocation _speretrace))
  ;[0.2232 0.227 0.2232] Sphere trace for kick and stabb
  (bind (_outhit _returnvalue_2) (Collision|SphereTraceByChannel _returnvalue _returnvalue 25.0 "TraceTypeQuery1" false 0 "None"))
  (if _returnvalue_2
    (if (Actor|ActorHasTag (.HitActor (Collision|BreakHitResult _outhit)) "Damageable")
      (Game|Damage|ApplyDamage (.HitActor (Collision|BreakHitResult _outhit)) (Variables|Default|GetBase%20Damage%20To%20Apply) 0 0)
      (Camera|PlayWorldCameraShake "/Game/Blueprints/Other/CS_HitCameraShake.CS_HitCameraShake_C" (.Location (Collision|BreakHitResult _outhit)) 0.0 2e+03)
      (CallFunction|PlaySwordHitSound)
      (Effects|SpawnEmitteratLocation "/Game/Assets/Particles/Blood/P_Blood_Splat_Cone.P_Blood_Splat_Cone" (.Location (Collision|BreakHitResult _outhit)) (Math|Rotator|MakeRotfromXY (.ImpactNormal (Collision|BreakHitResult _outhit)) (.ImpactNormal (Collision|BreakHitResult _outhit))) "0.400000,0.400000,0.400000"))))

(event Custom|StopCombo
  ;[0.2232 0.227 0.2232] Combo System
  ;;[0.2232 0.227 0.2232] Stop combo / attack
  (Variables|Default|SetIsAttacking false)
  (Variables|Default|SetAttackIndex 0))

(event Custom|Attack%204
  ;[0.2232 0.227 0.2232] Combo System
  ;;[0.2232 0.227 0.2232] Attack 1
  (Utilities|FlowControl|DoOnce false :!label _label
    (:Completed
      (Utilities|FlowControl|Delay 0.1)
      (Animation|Montage|PlayMontage (Variables|Default|GetCharacterMesh) "/Game/Assets/CharacterAnimations/SwordAttack/ANM_Attack3.ANM_Attack3"
        (:then
          (Variables|Default|SetAttackIndex 4)
          (goto _label Reset))))))

(event Custom|Play%20sword%20hit%20sound
  ;[0.2232 0.227 0.2232] play sword hit sound
  (Audio|PlaySoundatLocation "/Game/Assets/Audio/MeleeWapons/MS_SwordAttackHit.MS_SwordAttackHit" (Transformation|GetActorLocation (Components|GetOwner)) "0, 0, 0" 1.0 1.0 0.0 0 0 0 0))

(event Custom|Attack%202
  ;[0.2232 0.227 0.2232] Combo System
  ;;[0.2232 0.227 0.2232] Attack 2
  (Utilities|FlowControl|DoOnce false :!label _label
    (:Completed
      (Utilities|FlowControl|Delay 0.1)
      (Animation|Montage|PlayMontage (Variables|Default|GetCharacterMesh) "/Game/Assets/CharacterAnimations/SwordAttack/ANM_Attack2.ANM_Attack2"
        (:then
          (Variables|Default|SetAttackIndex 2)
          (goto _label Reset))))))

(event Custom|Attack1
  ;[0.2232 0.227 0.2232] Combo System
  ;;[0.2232 0.227 0.2232] Attack 1
  (Utilities|FlowControl|DoOnce false :!label _label
    (:Completed
      (Utilities|FlowControl|Delay 0.1)
      (Animation|Montage|PlayMontage (Variables|Default|GetCharacterMesh) "/Game/Assets/CharacterAnimations/SwordAttack/ANM_Attack1.ANM_Attack1"
        (:then
          (Variables|Default|SetAttackIndex 1)
          (goto _label Reset))))))

(event Custom|Attack%203
  ;[0.2232 0.227 0.2232] Combo System
  ;;[0.2232 0.227 0.2232] Attack 3
  (Utilities|FlowControl|DoOnce false :!label _label
    (:Completed
      (Utilities|FlowControl|Delay 0.1)
      (Animation|Montage|PlayMontage (Variables|Default|GetCharacterMesh) "/Game/Assets/CharacterAnimations/SwordAttack/ANM_Kick.ANM_Kick"
        (:then
          (Variables|Default|SetAttackIndex 3)
          (goto _label Reset))))))

(event Custom|Start%20Sword%20Trace
  ;[0.2232 0.227 0.2232] Sword Trace
  (bind _returnvalue (Utilities|Time|SetTimerbyEvent (delegate Custom|Sword%20Trace%20Loop) 0.001 true))
  (Variables|Default|SetSwordTraceLoop _returnvalue))

(event Input|EnhancedActionEvents|EnhancedInputActionIA_Attack
  (params (ActionValue :type Boolean) (ElapsedSeconds :type Float%20%28double-precision%29) (TriggeredSeconds :type Float%20%28double-precision%29) (InputAction :type Input%20Action%20Object%20Reference :default "/Game/Input/Actions/IA_Attack.IA_Attack"))
  ;[0.2232 0.227 0.2232] Combo System
  ;;[0.2232 0.227 0.2232] Attack input
  (:Started
    (if (Variables|Default|GetCanAttack)
      (CallFunction|SwordAttack))))

(event EventBeginPlay
  (bind _asbpc_player (Utilities|Casting|CastToBPC_Player (Components|GetOwner)))
  (Variables|Default|SetAs%20BPC%20Player _asbpc_player)
  (Variables|Default|SetCharacterMesh (Variables|/Script/Engine.Character|GetMesh _asbpc_player)))

(event EventTick
  (params (DeltaSeconds :type Float%20%28single-precision%29)))