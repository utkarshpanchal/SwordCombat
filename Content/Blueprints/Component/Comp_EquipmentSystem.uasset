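; Actor component that lets the player pick up weapons and stores their item data in a slot array.
; On begin play it casts its owner to BPC_Player and caches the follow camera.
; The interact input sphere-traces forward from the camera against WorldDynamic objects, with debug drawing.
; A hit BP_Weapon has its ItemData appended to StructSlots and is then destroyed.
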(event Input|EnhancedActionEvents|EnhancedInputActionIA_Interact
  (params (ActionValue :type Boolean) (ElapsedSeconds :type Float%20%28double-precision%29) (TriggeredSeconds :type Float%20%28double-precision%29) (InputAction :type Input%20Action%20Object%20Reference :default "/Game/Input/Actions/IA_Interact.IA_Interact"))
  (bind _follow_camera (Variables|Default|GetFollow%20Camera))
  (bind _returnvalue (Transformation|GetWorldLocation _follow_camera))
  ;[1 1 1] PickupTrace
  (:Started
    (bind (_outhit _returnvalue_2) (Collision|SphereTraceForObjects _returnvalue (+ _returnvalue (* (Math|Vector|GetForwardVector (Transformation|GetWorldRotation _follow_camera)) 1e+03)) 3e+01 (Utilities|Array|MakeArray "ObjectTypeQuery2") false 0 "ForDuration"))
    (if _returnvalue_2
      (bind _asbp_weapon (Utilities|Casting|CastToBP_Weapon (.HitActor (Collision|BreakHitResult _outhit))))
      (CallFunction|AddWeapons (Variables|/Game/Blueprints/GameplayMechanics/EquipmentSystem/Weapon_Blueprints/BP_Weapon.BP_Weapon_C|GetItemData _asbp_weapon))
      (Actor|DestroyActor _asbp_weapon))))

(event EventBeginPlay
  (bind _asbpc_player (Utilities|Casting|CastToBPC_Player (Components|GetOwner)))
  (Variables|Default|SetFollow%20Camera (Variables|/Game/Blueprints/Characters/BPC_Player.BPC_Player_C|GetFollowCamera _asbpc_player)))

(event EventTick
  (params (DeltaSeconds :type Float%20%28single-precision%29)))

(fn AddWeapons
  (params (NewItem :type Struct%20Slots%20Structure%20%28by%20ref%29))
  (Utilities|Array|Add (Variables|Default|GetStruct_Slots) NewItem))